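; BP_Porte is a door that opens once enough pressure plates ("plaques") are active.
; PlaqueActive and PlaqueDesactive adjust the active count and compare it to NbPlaqueBesoin.
; At or above that threshold, it plays a wooden opening sound and runs the OuvrirPorte timeline, which drives the Porte component's relative Z location.
; Below it, the timeline reverses.
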(event `PlaqueActive`
  (`/Engine/EditorBlueprintResources/StandardMacros.IncrementInt` (`self.NbPlaqueActive`)
    (:`  `
      (if (>= (`self.NbPlaqueActive`) (`self.NbPlaqueBesoin`))
        (`GameplayStatics.PlaySoundAtLocation` "/Game/Sons/new_wood_open.new_wood_open" (`self.K2_GetActorLocation`) (struct) 1.0 1.0 0.0 null null null null :!label _label)
        (bind (_direction _newtrack_0) (`Timeline|OuvrirPorte` :!label _label_2)
          (:`Update`
            (`SceneComponent.K2_SetRelativeLocation` (`self.Porte`) (`KismetMathLibrary.MakeVector` 0.0 0.0 _newtrack_0) false false)))
        (else
          (goto _label_2 :!via `Reverse`))))))

(event `PlaqueDesactive`
  (`/Engine/EditorBlueprintResources/StandardMacros.DecrementInt` (`self.NbPlaqueActive`)
    (:`  `
      (if (>= (`self.NbPlaqueActive`) (`self.NbPlaqueBesoin`))
        (goto _label)
        (else
          (goto _label_2 :!via `Reverse`))))))

(fn `UserConstructionScript`)