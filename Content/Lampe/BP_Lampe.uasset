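; BP_Lampe is a flashlight actor that trails the player camera and lights the view with a spotlight.
; Each tick it interpolates its location toward the camera position plus a camera-relative offset, and its rotation toward the camera rotation.
; Rotation interpolates at a slower speed than location.
; The Lampe input action toggles the SpotLight's visibility.
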(event `InputAction|Lampe`
  (params (Key :type "Key Structure"))
  (:`Pressed`
    (`SceneComponent.ToggleVisibility` (`self.SpotLight`) false)))

(event `self.ReceiveTick`
  (params (DeltaSeconds :type "Float (single-precision)"))
  (bind _returnvalue (`GameplayStatics.GetPlayerCameraManager` 0))
  (`self.K2_SetActorLocation` (`KismetMathLibrary.VInterpTo` (`self.K2_GetActorLocation`) (+ (`self.K2_GetActorLocation` _returnvalue) (`KismetMathLibrary.GreaterGreater_VectorRotator` (`self.CameraOffset`) (`self.K2_GetActorRotation` _returnvalue))) (`GameplayStatics.GetWorldDeltaSeconds`) 50.0))
  (`self.K2_SetActorRotation` (`KismetMathLibrary.RInterpTo` (`self.K2_GetActorRotation`) (`self.K2_GetActorRotation` (`GameplayStatics.GetPlayerCameraManager` 0)) (`GameplayStatics.GetWorldDeltaSeconds`) 10.0)))

(fn `UserConstructionScript`)