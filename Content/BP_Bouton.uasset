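; BP_Bouton is an interactable button that opens the garage doors linked to it by ID.
; On Interact, it searches all BP_PorteGarage actors for those whose PorteID matches its ButtonID and calls OuvrirPorte with the interacting player.
; For each match, it also switches the first player controller's view target to that door and destroys its own Box component.
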(event `/Game/BPI_Interact.Interact`
  (params (Player :type "Character Object Reference"))
  (bind _outactors (`GameplayStatics.GetAllActorsOfClass` "/Game/BP_PorteGarage.BP_PorteGarage_C"))
  (for _array_element _outactors
    (if (== (`/Game/BP_PorteGarage.PorteID` _array_element) (`self.ButtonID`))
      (`/Game/BP_PorteGarage.OuvrirPorte` _array_element Player)
      (`PlayerController.SetViewTargetWithBlend` (`GameplayStatics.GetPlayerController` 0) _array_element 0.0 "VTBlend_Linear" 0.0 false)
      (`ActorComponent.K2_DestroyComponent` (`self.Box`)))))

(fn `UserConstructionScript`)